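; Interactive sliding door, apparently for a bathroom, that toggles between closed and open each time its Activate event fires.
; BeginPlay caches the door component's world location as the start position.
; Activate plays or reverses a Timeline that sine-eases the whole scene root along a fixed world Y offset from that position.
; A PlayForward flag picks the direction and flips when the Timeline finishes.
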(event `self.ReceiveBeginPlay`
  (`parent.ReceiveBeginPlay`)
  (set `self.StartPos` (`SceneComponent.K2_GetComponentLocation` (`self.Bathroom_Sliding_Door`))))

(event `self.Activate`
  (bind _startpos (`self.StartPos`))
  (if (`self.playForward`)
    ;[1 1 1] Animation
    (bind (_direction _0_1) (`Timeline|Timeline` :!label _label)
      (:`Update`
        (`SceneComponent.K2_SetWorldLocation` (`self.DefaultSceneRoot`) (`|EaseFunction` "SinusoidalInOut" _0_1 _startpos (+ _startpos (0.0 80.0 0.0))) false false))
      (:`Finished`
        (set `self.playForward` (not (`self.playForward`)))))
    (else
      (goto _label :!via `Reverse`))))

(fn `UserConstructionScript`
  (`parent.UserConstructionScript`))