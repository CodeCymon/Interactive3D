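; BP_Blinds is an interactable window blinds actor that opens and closes four curtains when the player presses E nearby.
; Overlap sets the proximity flag and shows a "Window Blinds" screen prompt, which fades out and is removed on exit.
; A FlipFlop alternates forward and reverse playback on the curtain caches, pausing them after a fixed delay.
; A Playing flag blocks retriggering during the animation.
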(event `self.ReceiveBeginPlay`
  (bind _chaches (`self.Chaches`))
  (`self.EnableInput` (`GameplayStatics.GetPlayerController` 0))
  (`KismetArrayLibrary.Array_Add` _chaches (`self.front_left_curtain`))
  (`KismetArrayLibrary.Array_Add` _chaches (`self.front_right_curtian`))
  (`KismetArrayLibrary.Array_Add` _chaches (`self.back_right_curtain`))
  (`KismetArrayLibrary.Array_Add` _chaches (`self.back_left_curtain`)))

(event `self.ReceiveActorBeginOverlap`
  (params (OtherActor :type "Actor Object Reference"))
  ;[1 1 1] Prompt
  (set `self.isNear` true)
  (bind _returnvalue (`|CreateWidget` "/Game/UI/WB_ScreenPrompt.WB_ScreenPrompt_C"))
  (set `/Game/UI/WB_ScreenPrompt.prompt_text` "Window Blinds" _returnvalue)
  (`UserWidget.AddToViewport` _returnvalue 0))

(event `self.ReceiveActorEndOverlap`
  (params (OtherActor :type "Actor Object Reference"))
  ;[1 1 1] Prompt
  (set `self.isNear` false)
  (bind _fade (`/Game/UI/WB_ScreenPrompt.Fade` (stale `self.ReceiveActorBeginOverlap` _returnvalue)))
  (`UserWidget.PlayAnimation` (stale `self.ReceiveActorBeginOverlap` _returnvalue) _fade 0.0 1 "Reverse" 1.0 false)
  (`KismetSystemLibrary.Delay` (`WidgetAnimation.GetEndTime` _fade))
  (`Widget.RemoveFromParent` (stale `self.ReceiveActorBeginOverlap` _returnvalue)))

(event `UseCurtains`
  (bind _chaches (`self.Chaches`))
  (bind _chaches_2 (`self.Chaches`))
  (if (not (`self.playing`))
    (set `self.playing` true)
    (`/Engine/EditorBlueprintResources/StandardMacros.FlipFlop`
      (:`A`
        (for _index (range 4)
          (`GeometryCacheComponent.Play` (`|GetArrayItem` _chaches_2 _index))
          (`KismetSystemLibrary.Delay` 4.0)
          (for _index_2 (range 4)
            (`GeometryCacheComponent.Pause` (`|GetArrayItem` _chaches _index_2)))
          (set `self.playing` false)))
      (:`B`
        (for _index_3 (range 4)
          (`GeometryCacheComponent.PlayReversed` (`|GetArrayItem` _chaches_2 _index_3))
          (`KismetSystemLibrary.Delay` 4.0)
          (for _index_4 (range 4)
            (`GeometryCacheComponent.Pause` (`|GetArrayItem` _chaches _index_4)))
          (set `self.playing` false))))))

(event `Key|E` :consume false
  (params (Key :type "Key Structure"))
  ;[1 1 1] Keyboard Listener
  (:`Pressed`
    (if (`self.isNear`)
      (`self.UseCurtains`))))

(fn `UserConstructionScript`)