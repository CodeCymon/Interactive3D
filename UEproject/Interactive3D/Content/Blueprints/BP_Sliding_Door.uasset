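; Sliding bathroom door actor that the player opens and closes with E while inside its overlap area.
; Overlap sets a proximity flag and shows a screen prompt widget, which fades out by reversed animation before removal on exit.
; A FlipFlop alternately plays and reverses a timeline, easing the mesh sinusoidally between its start position and a fixed world-space Y offset.
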(event `self.ReceiveBeginPlay`
  (set `self.startPos` (`SceneComponent.K2_GetComponentLocation` (`self.Basestructure_S_Bathroom_Sliding_Door`)))
  (`self.EnableInput` (`GameplayStatics.GetPlayerController` 0)))

(event `self.ReceiveActorBeginOverlap`
  (params (OtherActor :type "Actor Object Reference"))
  (set `self.isNear` true)
  (bind _returnvalue (`|CreateWidget` "/Game/UI/WB_ScreenPrompt.WB_ScreenPrompt_C"))
  (`UserWidget.AddToViewport` _returnvalue 0))

(event `self.ReceiveActorEndOverlap`
  (params (OtherActor :type "Actor Object Reference"))
  (set `self.isNear` false)
  (bind _fade (`/Game/UI/WB_ScreenPrompt.Fade` (stale `self.ReceiveActorBeginOverlap` _returnvalue)))
  (`UserWidget.PlayAnimation` (stale `self.ReceiveActorBeginOverlap` _returnvalue) _fade 0.0 1 "Reverse" 1.0 false)
  (`KismetSystemLibrary.Delay` (`WidgetAnimation.GetEndTime` _fade))
  (`Widget.RemoveFromParent` (stale `self.ReceiveActorBeginOverlap` _returnvalue)))

(event `Key|E`
  (params (Key :type "Key Structure"))
  (:`Pressed`
    (if (`self.isNear`)
      (`self.Slide_Door`))))

(event `Slide_Door`
  (bind _startpos (`self.startPos`))
  (`/Engine/EditorBlueprintResources/StandardMacros.FlipFlop`
    (:`A`
      (bind (_direction _0_1) (`Timeline|Timeline` :!label _label)
        (:`Update`
          (`SceneComponent.K2_SetWorldLocation` (`self.Basestructure_S_Bathroom_Sliding_Door`) (`|EaseFunction` "SinusoidalInOut" _0_1 _startpos (+ _startpos (0.0 80.0 0.0))) false false))))
    (:`B`
      (goto _label :!via `Reverse`))))

(fn `UserConstructionScript`)