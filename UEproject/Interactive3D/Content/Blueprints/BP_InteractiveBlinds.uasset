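; BP_InteractiveBlinds is an interactive blinds actor that toggles four curtains with geometry cache animations.
; BeginPlay gathers the four curtain caches into an array.
; Activate uses a FlipFlop to alternate forward and reversed playback on all caches, then pauses them after a fixed delay.
; A Playing flag blocks new activations until the animation ends.
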(event `self.ReceiveBeginPlay`
  (bind _caches (`self.Caches`))
  (`parent.ReceiveBeginPlay`)
  ;[0.5387 0.8047 1] Adding All Geocaches to Array
  (`KismetArrayLibrary.Array_Add` _caches (`self.front_left_curtain`))
  (`KismetArrayLibrary.Array_Add` _caches (`self.front_right_curtian`))
  (`KismetArrayLibrary.Array_Add` _caches (`self.back_right_curtain`))
  (`KismetArrayLibrary.Array_Add` _caches (`self.back_left_curtain`)))

(event `self.Activate`
  (bind _caches (`self.Caches`))
  (bind _caches_2 (`self.Caches`))
  ;[0.1146 0.1146 0.1146] Toggle Blinds
  ;;[0 0 0] Prevent Use mid animation
  (if (not (`self.playing`))
    ;;[0 0 0] Toggle
    (set `self.playing` true)
    (`/Engine/EditorBlueprintResources/StandardMacros.FlipFlop`
      (:`A`
        ;;[0 0 0] Play every animation
        (for _index (range 4)
          (`GeometryCacheComponent.Play` (`|GetArrayItem` _caches _index))
          ;;[0 0 0] Wait
          (`KismetSystemLibrary.Delay` 4.0)
          ;;[0 0 0] Pause at End & Ready for new Interaction
          (for _index_2 (range 4)
            (`GeometryCacheComponent.Pause` (`|GetArrayItem` _caches_2 _index_2)))
          (set `self.playing` false)))
      (:`B`
        (for _index_3 (range 4)
          (`GeometryCacheComponent.PlayReversed` (`|GetArrayItem` _caches _index_3))
          (`KismetSystemLibrary.Delay` 4.0)
          (for _index_4 (range 4)
            (`GeometryCacheComponent.Pause` (`|GetArrayItem` _caches_2 _index_4)))
          (set `self.playing` false))))))

(fn `UserConstructionScript`
  (`parent.UserConstructionScript`))